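; Base pickup actor that puts an item into the player's backpack when the ThirdPersonCharacter touches it.
; Collision overlap calls PickUpItem, which asks the MyPlayerController's MyBackPack whether the item type and count fit.
; On success it adds the item, destroys itself and refreshes the character's bag UI.
; Nodes for maintaining the character's PickUpList are left unconnected, and end overlap does nothing.
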(event `self.CollisionComp.OnComponentBeginOverlap`
  (params (OverlappedComponent :type "PrimitiveComponent Object Reference") (OtherActor :type "Actor Object Reference") (OtherComp :type "PrimitiveComponent Object Reference") (OtherBodyIndex :type Integer) (bFromSweep :type Boolean) (SweepResult :type "HitResult Structure (by ref)"))
  (`self.PickUpItem` OtherActor))

(event `self.CollisionComp.OnComponentEndOverlap`
  (params (OverlappedComponent :type "PrimitiveComponent Object Reference") (OtherActor :type "Actor Object Reference") (OtherComp :type "PrimitiveComponent Object Reference") (OtherBodyIndex :type Integer)))

(event `PickUpItem`
  (params (otherActor :type "Actor Object Reference"))
  (bind _asthird_person_character (cast `/Game/ThirdPersonCPP/Blueprints/ThirdPersonCharacter` otherActor))
  (bind _asmy_player_controller (cast `MyPlayerController` (`Pawn.GetController` _asthird_person_character)))
  (bind _mybackpack (`MyPlayerController.myBackPack` _asmy_player_controller))
  (bind _returnvalue (`BackPackComponent.CanAddItem` _mybackpack (`self.ItemTypeId`) (`self.ItemCount`)))
  (if _returnvalue
    (`BackPackComponent.AddItem` _mybackpack (`self.ItemTypeId`) (`self.ItemCount`) otherActor)
    (`self.K2_DestroyActor` self)
    (`/Game/ThirdPersonCPP/Blueprints/ThirdPersonCharacter.RefreshBagUI` _asthird_person_character)))

(fn `UserConstructionScript`)